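; Level generator actor that builds a dungeon from a grid of tile data when BuildLevel is called.
; It destroys existing pieces and resizes DungeonTiles whenever the array length differs from MapSizeX times MapSizeY.
; Each enabled tile reuses or spawns an attached DungeonPiece at its raised grid position, then passes it the wall data and calls Update.
; Pieces on disabled tiles are destroyed, so rebuilds update the existing layout in place.
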(event EventBeginPlay)

(event Collision|EventActorBeginOverlap
  (params (OtherActor :type Actor%20Object%20Reference)))

(event EventTick
  (params (DeltaSeconds :type Float%20%28single-precision%29)))

(event EventBuildLevel
  (bind _dungeontiles (Variables|Default|GetDungeonTiles))
  (bind _mapsizex (Variables|Default|GetMapSizeX))
  (bind _dungeontiles_2 (Variables|Default|GetDungeonTiles))
  (bind _mapsizey (Variables|Default|GetMapSizeY))
  (bind _returnvalue (* _mapsizex _mapsizey))
  (Development|PrintString "Build Level called")
  (Utilities|FlowControl|Sequence
    (:then_0
      ;[1 1 1 0.136] Resize Array if necessary
      (if (== _returnvalue (Utilities|Array|Length _dungeontiles_2))
        (Development|PrintString "Proper Size")
        (else
          (for _array_element _dungeontiles_2
            (Actor|DestroyActor _array_element))
          (Utilities|Array|Resize _dungeontiles_2 _returnvalue)
          (Development|PrintString "Had to resize"))))
    (:then_1
      ;[1 1 1 0.17] Create, Delete and update tile actors
      (for (_array_element_2 _array_index) (Variables|Default|GetTiles)
        (if (.Enabled (Utilities|Struct|Break _array_element_2))
          (if (Utilities|IsValid (Utilities|Array|Get(acopy) _dungeontiles _array_index))
            (Transformation|SetActorLocation (Utilities|Array|Get(acopy) _dungeontiles _array_index) (+ (CallFunction|GetTileWorldPosition _array_index) "0, 0,100.000000") false false)
            (else
              (bind _returnvalue_2 (Game|SpawnActorfromClass "/Game/Trash/DungeonPiece.DungeonPiece_C" (Math|Conversions|ToTransform(Vector) (+ (CallFunction|GetTileWorldPosition _array_index) "0, 0,100.000000")) "Undefined" self 0 0))
              (Utilities|Array|SetArrayElem _dungeontiles _array_index _returnvalue_2)
              (Transformation|AttachComponentToComponent _returnvalue_2 (Variables|Transformation|GetRootComponent) "None" "KeepWorld" "KeepWorld" "KeepWorld" false)))
          (bind _asdungeon_piece (Utilities|Casting|CastToDungeonPiece (Utilities|Array|Get(acopy) _dungeontiles _array_index)))
          (Variables|/Game/Trash/DungeonPiece.DungeonPiece_C|SetWallArray _asdungeon_piece (.Walls (Utilities|Struct|Break _array_element_2)))
          (Default|Update _asdungeon_piece)
          (elif (Utilities|IsValid (Utilities|Array|Get(acopy) _dungeontiles _array_index))
            (Actor|DestroyActor (Utilities|Array|Get(acopy) _dungeontiles _array_index))))))))

(fn ConstructionScript)