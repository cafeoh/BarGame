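; DungeonPiece is a modular dungeon tile that configures its floor and four walls from a WallArray.
; Update, run from the Construction Script, hides each side or shows it with a wall or door mesh, toggling collision to match.
; Dynamic material instances receive ambient occlusion parameters: walls from their neighboring sides, the floor from all four sides.
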(event Custom|Update
  (bind _wallarray (Variables|Default|GetWallArray))
  (Utilities|FlowControl|Sequence
    (:then_0
      (if (== (Utilities|Array|Length _wallarray) 4)
        (for (_array_element _array_index) _wallarray
          (switch int (Math|Conversions|ToInteger(Byte) _array_element)
            (:0
              (Rendering|SetVisibility (Utilities|Array|Get(acopy) (Utilities|Array|MakeArray (Variables|Default|GetNorthWall) (Variables|Default|GetEastWall) (Variables|Default|GetSouthWall) (Variables|Default|GetWestWall)) _array_index) false true)
              (Collision|SetCollisionEnabled (Utilities|Array|Get(acopy) (Utilities|Array|MakeArray (Variables|Default|GetNorthWall) (Variables|Default|GetEastWall) (Variables|Default|GetSouthWall) (Variables|Default|GetWestWall)) _array_index) "NoCollision"))
            (:1
              (Components|StaticMesh|SetStaticMesh (Utilities|Array|Get(acopy) (Utilities|Array|MakeArray (Variables|Default|GetNorthWall) (Variables|Default|GetEastWall) (Variables|Default|GetSouthWall) (Variables|Default|GetWestWall)) _array_index) "/Game/Meshes/NewWall.NewWall")
              (Rendering|SetVisibility (Utilities|Array|Get(acopy) (Utilities|Array|MakeArray (Variables|Default|GetNorthWall) (Variables|Default|GetEastWall) (Variables|Default|GetSouthWall) (Variables|Default|GetWestWall)) _array_index) true true :!label _label)
              (Collision|SetCollisionEnabled (Utilities|Array|Get(acopy) (Utilities|Array|MakeArray (Variables|Default|GetNorthWall) (Variables|Default|GetEastWall) (Variables|Default|GetSouthWall) (Variables|Default|GetWestWall)) _array_index) "QueryAndPhysics")
              ;[1 1 1] Set walls AO
              (bind _returnvalue (Rendering|Material|CreateDynamicMaterialInstance "/Game/Materials/MI_Wall.MI_Wall" :!class /Script/Engine.KismetMaterialLibrary))
              (Rendering|Material|SetScalarParameterValue _returnvalue "Left AO" (Math|Conversions|ToFloat(Boolean) (!= (Utilities|Array|Get(acopy) _wallarray (Math|Conversions|ToInteger(Byte) (Class|KismetMathLibrary|PercentByteByte (- (Math|Conversions|ToByte(Integer) _array_index) 1) 4))) 0)) :!class /Script/Engine.MaterialInstanceDynamic)
              (Rendering|Material|SetScalarParameterValue _returnvalue "Right AO" (Math|Conversions|ToFloat(Boolean) (!= (Utilities|Array|Get(acopy) _wallarray (Math|Conversions|ToInteger(Byte) (Class|KismetMathLibrary|PercentByteByte (+ (Math|Conversions|ToByte(Integer) _array_index) 1) 4))) 0)) :!class /Script/Engine.MaterialInstanceDynamic)
              (Rendering|Material|SetMaterial (Utilities|Array|Get(acopy) (Utilities|Array|MakeArray (Variables|Default|GetNorthWall) (Variables|Default|GetEastWall) (Variables|Default|GetSouthWall) (Variables|Default|GetWestWall)) _array_index) 0 _returnvalue))
            (:2
              (Components|StaticMesh|SetStaticMesh (Utilities|Array|Get(acopy) (Utilities|Array|MakeArray (Variables|Default|GetNorthWall) (Variables|Default|GetEastWall) (Variables|Default|GetSouthWall) (Variables|Default|GetWestWall)) _array_index) "/Game/Meshes/NewDoor.NewDoor")
              (goto _label))))
        ;[1 1 1] Set floor AO
        (bind _returnvalue_2 (Rendering|Material|CreateDynamicMaterialInstance "/Game/Materials/MI_Floor.MI_Floor" :!class /Script/Engine.KismetMaterialLibrary))
        (for (_array_element_2 _array_index_2) _wallarray
          (Rendering|Material|SetScalarParameterValue _returnvalue_2 (Utilities|Array|Get(acopy) (Utilities|Array|MakeArray "North AO" "East AO" "South AO" "West AO") _array_index_2) (Math|Float|Clamp(Float) (Math|Conversions|ToFloat(Byte) _array_element_2)) :!class /Script/Engine.MaterialInstanceDynamic))
        (Rendering|Material|SetMaterial (Variables|Default|GetFloor) 0 _returnvalue_2)
        (else
          (Development|PrintString "Walls array in tile isn't size 4!"))))))

(event EventBeginPlay)

(event Collision|EventActorBeginOverlap
  (params (OtherActor :type Actor%20Object%20Reference)))

(event EventTick
  (params (DeltaSeconds :type Float%20%28single-precision%29)))

(fn ConstructionScript
  (CallFunction|Update))