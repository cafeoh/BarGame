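; VR-grippable test tube holding a LiquidUnit content, with simulated sloshing and pouring into other test tubes.
; A damped inertia point tilts a fill-based plane that slices a procedural copy of the liquid mesh.
; Uncapped outflow depends on the sliced exit area; a downward trace picks transfer or spill and places the stream mesh.
; Updates run while physics is awake, with heavy liquid work gated by a timed wake state.
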(event Custom|Update%20Liquid
  (bind _capped (Variables|Default|GetCapped))
  (bind _plug (Variables|Default|GetPlug))
  (Utilities|FlowControl|Sequence
    (:then_0
      (CallFunction|UpdateLiquidInertia)
      (if (or (Class|PrimitiveComponent|IsAnyRigidBodyAwake (Variables|Default|GetContainer)) (> (Math|Vector|VectorLength (Variables|Default|GetLiquidVelocity)) 0.01))
        (CallFunction|Wake))
      (Rendering|SetVisibility _plug _capped false)
      (Collision|SetCollisionEnabled _plug (select _capped "QueryAndPhysics" "NoCollision")))
    (:then_1
      (Rendering|Debug|FlushPersistentDebugLines)
      (if (Utilities|IsAwake)
        ;[1 0 0.2358 1 16] Liquid Heavylifting
        (CallFunction|HandleLiquidSystem)
        (Rendering|Debug|DrawDebugPoint (Transformation|GetWorldLocation (Variables|Default|GetContainer)) 1.0 "(R=0.000000,G=1.000000,B=0.277806,A=1.000000)" 0.0)))))

(event EventTick
  (params (DeltaSeconds :type Float%20%28single-precision%29))
  (bind _sourcetextroot (Variables|Default|GetSourceTextRoot))
  (Transformation|SetWorldRotation _sourcetextroot (Math|Rotator|MakeRotator 0.0 0.0 (.Yaw (Math|Rotator|BreakRotator (Math|Rotator|Lerp(Rotator) (Transformation|GetWorldRotation _sourcetextroot) (Math|Rotator|FindLookatRotation (Transformation|GetWorldLocation _sourcetextroot) (Transformation|GetActorLocation (Game|Player|GetPlayerPawn 0))) 0.5 true)))) false false)
  (if (Class|PrimitiveComponent|IsAnyRigidBodyAwake (Variables|Default|GetContainer))
    (CallFunction|UpdateLiquid)))

(fn ConstructionScript
  (Utilities|IsValid (Variables|Default|GetContent)
    (:Is%20Valid
      _)
    (:Is%20Not%20Valid
      (bind _returnvalue (Game|ConstructObjectfromClass "/Game/Blueprints/LiquidUnit.LiquidUnit_C" self))
      (bind _output_get (Variables|Default|SetContent _returnvalue))))
  (Variables|/Game/Blueprints/LiquidUnit.LiquidUnit_C|SetSource _output_get (Variables|Default|GetSource))
  (Rendering|SetVisibility (Variables|Default|GetSourceTextRoot) (Variables|Default|GetSource) true)
  (bind _returnvalue_2 (Rendering|Material|CreateDynamicMaterialInstance (Variables|Default|GetMaterialInstance) "/Game/Materials/MI_Liquid.MI_Liquid" :!class /Script/Engine.KismetMaterialLibrary))
  (bind _output_get_2 (Variables|Default|SetMaterialInstance _returnvalue_2))
  (Variables|Default|SetLiquidInertia (Transformation|GetWorldLocation (Variables|Default|GetContainer)))
  (Utilities|FlowControl|Sequence
    (:then_0
      (bind _returnvalue_3 (AddComponent|AddProceduralMeshComponent false))
      (bind _output_get_3 (Variables|Default|SetProcedural%20Liquid _returnvalue_3))
      (Rendering|Material|SetMaterial _output_get_3 0 _output_get_2))
    (:then_1
      (CallFunction|UpdateLiquid))))

(fn UpdateLiquidInertia
  (bind _returnvalue (Utilities|Time|GetWorldDeltaSeconds))
  (bind _returnvalue_2 (* _returnvalue 1.0))
  (bind _output_get (Variables|Default|SetLiquidVelocity (/ (+ (* (- (Transformation|GetWorldLocation (Variables|Default|GetContainer)) (Variables|Default|GetLiquidInertia)) (* _returnvalue_2 1.0)) (Variables|Default|GetLiquidVelocity)) (+ (* _returnvalue_2 1e+01) 1.0))))
  (bind _output_get_2 (Variables|Default|SetLiquidInertia (+ (* _output_get (* _returnvalue_2 5e+02)) (Variables|Default|GetLiquidInertia))))
  (Rendering|Debug|DrawDebugPoint _output_get_2 5.0 "(R=0.109375,G=0.070750,B=0.000000,A=1.000000)" 0.0)
  (return))

(fn AddLiquid
  (bind _content (Variables|Default|GetContent))
  (Default|AddConcentrates _content (Variables|Default|GetComponentsToAdd) 1.0)
  (Variables|/Game/Blueprints/LiquidUnit.LiquidUnit_C|SetVolume _content (+ (Variables|/Game/Blueprints/LiquidUnit.LiquidUnit_C|GetVolume _content) 1e+01))
  (CallFunction|UpdateLiquid))

(fn GetLiquidPlane
  (bind _content (Variables|Default|GetContent))
  (bind _container (Variables|Default|GetContainer))
  (bind _capacity (Variables|Default|GetCapacity))
  (bind _liquidinertia (Variables|Default|GetLiquidInertia))
  (bind _returnvalue (Transformation|GetWorldLocation _container))
  (bind _volume (Variables|/Game/Blueprints/LiquidUnit.LiquidUnit_C|GetVolume _content))
  (bind _returnvalue_2 (- _returnvalue _liquidinertia))
  (bind _returnvalue_3 (/ _volume _capacity))
  (bind _returnvalue_4 (+ _returnvalue_2 "0, 0,10.000000"))
  (bind _returnvalue_5 (Math|Vector|Lerp(Vector) "0, 0,1.000000" _returnvalue_4 _returnvalue_3))
  (bind _returnvalue_6 (Math|Vector|Normalize _returnvalue_5))
  (bind _returnvalue_7 (Class|LiquidSystem|GetVolumetricSlicingPlane (Variables|Default|GetLiquid) _returnvalue_3 _returnvalue_6))
  (return _returnvalue_7 _returnvalue_6))

(fn PrintContent
  (Default|PrintContent (Variables|Default|GetContent)))

(fn HandleLiquidSystem
  (bind _exit (Variables|Default|GetExit))
  (bind _content (Variables|Default|GetContent))
  (bind _content_2 (Variables|Default|GetContent))
  (bind _content_3 (Variables|Default|GetContent))
  (bind _procedural_liquid (Variables|Default|GetProcedural%20Liquid))
  (bind _pouringliquid (Variables|Default|GetPouringLiquid))
  (bind _materialinstance (Variables|Default|GetMaterialInstance))
  (bind _volume (Variables|/Game/Blueprints/LiquidUnit.LiquidUnit_C|GetVolume _content))
  (bind _volume_2 (Variables|/Game/Blueprints/LiquidUnit.LiquidUnit_C|GetVolume _content_3))
  (bind _returnvalue (> _volume_2 0.0))
  (Rendering|SetVisibility (Variables|Default|GetProcedural%20Liquid) _returnvalue true)
  (Rendering|SetVisibility (Variables|Default|GetPouringLiquid) _returnvalue true)
  (if _returnvalue
    (Utilities|FlowControl|Sequence
      (:then_0
        ;[1 1 1] Liquid & Container
        (Default|UpdateMaterialInstance (Variables|Default|GetContent) _materialinstance)
        (Rendering|Material|SetMaterial (Variables|Default|GetLiquid) 0 _materialinstance)
        (Class|KismetProceduralMeshLibrary|CopyProceduralMeshfromStaticMeshComponent (Variables|Default|GetLiquid) 0 _procedural_liquid false)
        (bind (_planeposition _planenormal) (CallFunction|GetLiquidPlane))
        (Rendering|SetTranslucentSortPriority _procedural_liquid 5)
        (bind _output_get (Variables|Default|SetPlaneNormal _planenormal))
        (bind _output_get_2 (Variables|Default|SetPlanePosition _planeposition))
        (Class|KismetProceduralMeshLibrary|SliceProceduralMesh _procedural_liquid _output_get_2 (* _output_get -1.0) false "UseLastSectionForCap" (Rendering|Material|GetMaterial _procedural_liquid 0)))
      (:then_1
        ;[1 1 1] Pouring logic
        (bind _returnvalue_2 (Class|LiquidSystem|GetSlicedExitArea _exit (Variables|Default|GetPlanePosition) (Variables|Default|GetPlaneNormal)))
        (Variables|Default|SetLiquidExitPoint (.OutPointOnBody (Collision|GetClosestPointonCollision _exit (- (.Origin (Collision|GetComponentBounds _exit)) "0, 0,5.000000") "None")))
        (bind _output_get_3 (Variables|Default|SetLiquid%20Outpour (Math|Float|Clamp(Float) (* (* (Math|Conversions|ToFloat(Boolean) (not (Variables|Default|GetCapped))) (Utilities|ComputeOutpour _returnvalue_2 1e+02 1e+02 _exit)) (Utilities|Time|GetWorldDeltaSeconds)) (- _volume (Variables|Default|GetCapacity)) _volume)))
        (Rendering|SetVisibility (Variables|Default|GetPouringLiquid) (> _output_get_3 0.0) false)
        (if (> _output_get_3 0.0)
          (CallFunction|Wake)
          (bind _outhit (Collision|LineTraceByChannel (Variables|Default|GetLiquidExitPoint) (+ (Variables|Default|GetLiquidExitPoint) "0, 0,-1000.000000") "TraceTypeQuery1" true 0 "None" true "(R=1.000000,G=0.000000,B=0.000000,A=1.000000)" "(R=0.000000,G=0.000000,B=0.000000,A=1.000000)" 0.1))
          (Variables|Default|SetLiquidImpactPoint (.ImpactPoint (Collision|BreakHitResult _outhit)))
          (bind _ascontainer (Utilities|Casting|CastToTestTube (.HitActor (Collision|BreakHitResult _outhit)))
            (:then
              (if (> (Math|Vector|DotProduct (- (.Origin (Collision|GetComponentBounds (Variables|TestTube_C|GetContainer _ascontainer))) (Variables|Default|GetLiquidImpactPoint)) (.ImpactNormal (Collision|BreakHitResult _outhit))) 0.0)
                (Default|PourIntoContainer _content_2 (Variables|TestTube_C|GetContent _ascontainer) (Variables|Default|GetLiquid%20Outpour))
                (CallFunction|UpdateLiquid _ascontainer)
                (CallFunction|Wake _ascontainer)
                (else
                  (Default|PourOut _content_2 (Variables|Default|GetLiquid%20Outpour) :!label _label))))
            (:CastFailed
              (goto _label)))))
      (:then_2
        ;[1 1 1] Pouring visuals
        (Rendering|SetVisibility (Variables|Default|GetPouringLiquid) (> (Variables|Default|GetLiquid%20Outpour) 0.0) false)
        (Effects|Components|ParticleSystem|SetEmitterEnable (Variables|Default|GetSplash) "None" (> (Variables|Default|GetLiquid%20Outpour) 0.0))
        (if (> (Variables|Default|GetLiquid%20Outpour) 0.0)
          (Rendering|Material|SetMaterial _pouringliquid 0 (Rendering|Material|GetMaterial (Variables|Default|GetLiquid) 0))
          (Transformation|SetWorldTransform _pouringliquid (Math|Transform|MakeTransform (Math|Vector|Lerp(Vector) (Variables|Default|GetLiquidExitPoint) (Variables|Default|GetLiquidImpactPoint) 0.5) "0, 0, 0" (/ (Math|Vector|MakeVector (* (Math|Float|Sqrt (Variables|Default|GetLiquid%20Outpour)) 0.5) (* (Math|Float|Sqrt (Variables|Default|GetLiquid%20Outpour)) 0.5) (Math|Vector|VectorLength (- (Variables|Default|GetLiquidExitPoint) (Variables|Default|GetLiquidImpactPoint)))) 1e+02)) false false))))))

(fn Wake
  (Variables|Default|SetLastAwake (Utilities|Time|GetGameTimeinSeconds)))

(fn AdvancedGripSettings
  (return ""))

(fn ClosestGripSlotinRange
  (params (WorldLocation :type Vector :default "0, 0, 0") (bSecondarySlot :type Boolean) (CallingController :type Grip%20Motion%20Controller%20Component%20Object%20Reference) (OverridePrefix :type Name :default "None"))
  (return false ""))

(fn DenyGripping
  (return false))

(fn GetGripStiffnessandDamping
  (return 0.0 0.0))

(fn GetInteractionSettings
  (return ""))

(fn GetPrimaryGripType
  (params (bIsSlot :type Boolean))
  (return "InteractiveCollisionWithPhysics"))

(fn GripBreakDistance
  (return 0.0))

(fn GripLateUpdateSetting
  (return "LateUpdatesAlwaysOn"))

(fn GripMovementReplicationType
  (return "KeepOriginalMovement"))

(fn IsHeld
  (return 0 false))

(fn IsInteractible
  (return false))

(fn SecondaryGripType
  (return "SG_None"))

(fn SimulateonDrop
  (return false))

(fn TeleportBehavior
  (return "TeleportAllComponents"))