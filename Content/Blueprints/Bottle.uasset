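; Bottle actor for a liquid-pouring system, selectable as a wine or flat bottle through its Type.
; The construction script assigns container, liquid, exit and label meshes and sets the capacity for that type, then runs the parent construction script.
; Outpour amount is the smaller of the Exit and NeckExit areas sliced by a plane, so the tighter opening limits the flow.
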(event EventBeginPlay)

(event Collision|EventActorBeginOverlap
  (params (OtherActor :type Actor%20Object%20Reference)))

(event EventTick
  (params (DeltaSeconds :type Float%20%28single-precision%29))
  (|CallParentFunction DeltaSeconds) ; This node is disabled and will not be called.\nDrag off pins to build functionality.
)

(fn ConstructionScript
  (bind _container (Variables|Default|GetContainer))
  (bind _label (Variables|Default|GetLabel))
  (bind _liquid (Variables|Default|GetLiquid))
  (bind _exit (Variables|Default|GetExit))
  (Utilities|FlowControl|Sequence
    (:then_0
      (switch Utilities|FlowControl|Switch|SwitchonContainerType (Variables|Default|GetType)
        (:NewEnumerator2
          (Components|StaticMesh|SetStaticMesh _container "/Game/Meshes/WineBottle_Container.WineBottle_Container")
          (Components|StaticMesh|SetStaticMesh _liquid "/Game/Meshes/WineBottle_Liquid.WineBottle_Liquid")
          (Components|StaticMesh|SetStaticMesh _exit "/Game/Meshes/WineBottle_Exit.WineBottle_Exit")
          (Components|StaticMesh|SetStaticMesh _label "/Game/Meshes/WineBottle_Label.WineBottle_Label")
          (Variables|Default|SetCapacity 8e+02))
        (:NewEnumerator3
          (Components|StaticMesh|SetStaticMesh _container "/Game/Meshes/FlatBottle_Container.FlatBottle_Container")
          (Components|StaticMesh|SetStaticMesh _liquid "/Game/Meshes/FlatBottle_Liquid.FlatBottle_Liquid")
          (Components|StaticMesh|SetStaticMesh _exit "/Game/Meshes/FlatBottle_Exit.FlatBottle_Exit")
          (Components|StaticMesh|SetStaticMesh _label "/Game/Meshes/FlatBottle_Label.FlatBottle_Label")
          (Variables|Default|SetCapacity 9.2e+02))))
    (:then_1
      (|CallParentFunction))))

(fn GetPunctualOutpourAmount
  (bind _planeposition (Variables|Default|GetPlanePosition))
  (bind _planenormal (Variables|Default|GetPlaneNormal))
  (bind _returnvalue (Class|LiquidSystem|GetSlicedExitArea (Variables|Default|GetExit) _planeposition _planenormal))
  (bind _returnvalue_2 (Class|LiquidSystem|GetSlicedExitArea (Variables|Default|GetNeckExit) _planeposition _planenormal))
  (return (Math|Float|Min(Float) _returnvalue_2 _returnvalue)))