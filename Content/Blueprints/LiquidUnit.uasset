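; LiquidUnit models a volume of mixed liquids that can be filled, poured into another unit or emptied.
; AddLiquid merges entries by type and grows Volume, while PourOut scales each entry proportionally and recomputes Volume.
; PourIntoContainer sends scaled portions to the recipient's AddLiquid, calling PourOut inside its per-liquid loop.
; AddConcentrates blends Color and MRO by volume weight, and UpdateMaterialInstance writes both to a material instance.
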(fn UpdateMaterialInstance
  (params (MaterialInstanceIn :type Material%20Instance%20Dynamic%20Object%20Reference%20%28by%20ref%29))
  (Rendering|Material|SetVectorParameterValue MaterialInstanceIn "MRO" (Math|Conversions|ToLinearColor(Vector) (Variables|Default|GetMRO)) :!class /Script/Engine.MaterialInstanceDynamic)
  (Rendering|Material|SetVectorParameterValue MaterialInstanceIn "Color" (Math|Conversions|ToLinearColor(Vector) (Variables|Default|GetColor)) :!class /Script/Engine.MaterialInstanceDynamic)
  (return))

(fn PourIntoContainer
  (params (Recipient :type Liquid%20Unit%20Object%20Reference%20%28by%20ref%29) (Quantity :type Float%20%28single-precision%29))
  (for _array_element (Variables|Default|GetLiquids)
    (Variables|/Game/Blueprints/Liquid.Liquid_C|SetQuantity _array_element (* (Variables|/Game/Blueprints/Liquid.Liquid_C|GetQuantity _array_element) (/ Quantity (Variables|Default|GetVolume))))
    (CallFunction|AddLiquid Recipient _array_element)
    (CallFunction|PourOut Quantity)))

(fn PourOut
  (params (QuantityOut :type Float%20%28single-precision%29))
  (bind _liquids (Variables|Default|GetLiquids))
  (for (_array_element _array_index) _liquids
    (bind _output_get (Variables|/Game/Blueprints/Liquid.Liquid_C|SetQuantity _array_element (|((({EA9AAF71-460E-2104-2C34-52BC6AB0ECAF}-QuantityOut)/{EA9AAF71-460E-2104-2C34-52BC6AB0ECAF})*Quantity) QuantityOut (Variables|/Game/Blueprints/Liquid.Liquid_C|GetQuantity _array_element))))
    (LocalVariables|SetNewVolume (+ _output_get (LocalVariables|GetNewVolume)))
    (Utilities|Array|SetArrayElem _liquids _array_index _array_element))
  (Variables|Default|SetVolume (LocalVariables|GetNewVolume)))

(fn PrintContent
  (Development|PrintString 0 (Utilities|String|Append "Volume :" (Utilities|String|ToString(Float) (Variables|Default|GetVolume)) "ml"))
  (for _array_element (Variables|Default|GetLiquids)
    (Development|PrintString 0 (Utilities|String|Append (Utilities|String|EnumtoString (Variables|/Game/Blueprints/Liquid.Liquid_C|GetType _array_element)) " : " (Utilities|String|ToString(Float) (Variables|/Game/Blueprints/Liquid.Liquid_C|GetQuantity _array_element))))))

(fn AddConcentrates
  (params (Color :type Vector) (MRT :type Vector) (Quantity :type Float%20%28single-precision%29))
  (if (> Quantity 0.0)
    (Variables|Default|SetColor (+ (* (Variables|Default|GetColor) (/ (Variables|Default|GetVolume) (+ Quantity (Variables|Default|GetVolume)))) (* Color (- 1.0 (/ (Variables|Default|GetVolume) (+ Quantity (Variables|Default|GetVolume)))))))
    (Variables|Default|SetMRO (+ (* (Variables|Default|GetMRO) (/ (Variables|Default|GetVolume) (+ Quantity (Variables|Default|GetVolume)))) (* MRT (- 1.0 (/ (Variables|Default|GetVolume) (+ Quantity (Variables|Default|GetVolume)))))))
    (Variables|Default|SetVolume (+ Quantity (Variables|Default|GetVolume)))))

(fn EmptyOut
  (Variables|Default|SetVolume 0.0)
  (Utilities|Array|Clear (Variables|Default|GetLiquids)))

(fn AddLiquid
  (params (Liquid :type Liquid%20Object%20Reference))
  (bind _quantity (Variables|/Game/Blueprints/Liquid.Liquid_C|GetQuantity Liquid))
  (bind _liquids (Variables|Default|GetLiquids))
  (if (> _quantity 0.0)
    (bind (_array_element _array_index) (Utilities|Array|ForEachLoopwithBreak _liquids :!label _label)
      (:LoopBody
        (if (Utilities|Enum|Equal(Enum) (Variables|/Game/Blueprints/Liquid.Liquid_C|GetType _array_element) (Variables|/Game/Blueprints/Liquid.Liquid_C|GetType Liquid))
          (LocalVariables|SetLiquidExists true)
          (Default|Merge _array_element Liquid)
          (Utilities|Array|SetArrayElem _liquids _array_index _array_element)
          (goto _label Break)))
      (:Completed
        (Variables|Default|SetVolume (+ _quantity (Variables|Default|GetVolume)))
        (if (not (LocalVariables|GetLiquidExists))
          (Utilities|Array|Add (Variables|Default|GetLiquids) Liquid))))))