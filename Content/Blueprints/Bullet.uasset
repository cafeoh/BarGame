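; Bullet projectile actor that damages what it hits, pushes physics objects and destroys itself on impact.
; The construction script creates a dynamic material on the Sphere mesh.
; Tick uses the remaining lifespan to shift the material's red channel and compound a shrinking scale during the final second.
; On hit, it applies a forward impulse at the impact point to simulating components, then calls DestroyActor before ApplyDamage.
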(event OnComponentHit(SphereCollision)
  (params (HitComponent :type Primitive%20Component%20Object%20Reference) (OtherActor :type Actor%20Object%20Reference) (OtherComp :type Primitive%20Component%20Object%20Reference) (NormalImpulse :type Vector :default "0, 0, 0") (Hit :type Hit%20Result%20Structure%20%28by%20ref%29))
  (bind (_bblockinghit _binitialoverlap _time _location _impactpoint _normal _impactnormal _physmat _hitactor _hitcomponent) (Collision|BreakHitResult Hit))
  (if (Physics|IsSimulatingPhysics _hitcomponent "None")
    (Physics|AddImpulseatLocation _hitcomponent (* (Math|Vector|GetForwardVector (Variables|Default|GetSphere)) 2e+03) _impactpoint "None"))
  (Actor|DestroyActor)
  (Game|Damage|ApplyDamage _hitactor 1.0 0 0))

(event EventTick
  (params (DeltaSeconds :type Float%20%28single-precision%29))
  (bind _returnvalue (Actor|GetLifeSpan))
  (bind _sphere (Variables|Default|GetSphere))
  (Rendering|Material|SetVectorParameterValue (Variables|Default|GetDynamicMaterial) "DiffuseColor" (Math|Color|MakeColor (- 1.0 _returnvalue) 0.0 0.0) :!class /Script/Engine.MaterialInstanceDynamic)
  (Transformation|SetWorldScale3D _sphere (* (Transformation|GetWorldScale _sphere) (Math|Float|Clamp(Float) _returnvalue))))

(fn ConstructionScript
  (bind _returnvalue (Rendering|Material|CreateDynamicMaterialInstance (Variables|Default|GetSphere) 0 0 :!class /Script/Engine.PrimitiveComponent))
  (Variables|Default|SetDynamicMaterial _returnvalue))