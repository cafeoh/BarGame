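; SkullTube is a dispenser actor that launches a new SkullBP out of its cylinder when player 0 presses E.
; Tick polls the key, then spawns the skull at the cylinder, fired along its up vector with Alive off and a custom collision channel set to overlap.
; Once the skull no longer overlaps the cylinder, that channel is set to block, the skull becomes Alive and the tube is ready again.
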(event EventBeginPlay)

(event Collision|EventActorBeginOverlap
  (params (OtherActor :type Actor%20Object%20Reference)))

(event EventTick
  (params (DeltaSeconds :type Float%20%28single-precision%29))
  (bind _cylinder (Variables|Default|GetCylinder))
  (bind _returnvalue (Math|Vector|GetUpVector _cylinder))
  (if (Variables|Default|GetReady)
    (if (Game|Player|WasInputKeyJustPressed (Game|GetPlayerController 0) "E")
      (bind _returnvalue_2 (Game|SpawnActorfromClass "/Game/Blueprints/SkullBP.SkullBP_C" (Math|Transform|MakeTransform (Transformation|GetWorldLocation _cylinder) (Math|Conversions|RotationFromXVector _returnvalue)) "Undefined" 0 0))
      (bind _output_get (Variables|Default|SetFreshSkull _returnvalue_2))
      (Variables|/Game/Blueprints/SkullBP.SkullBP_C|SetAlive _output_get false)
      (Collision|SetCollisionResponsetoChannel (Variables|/Game/Blueprints/SkullBP.SkullBP_C|GetSkull _output_get) "ECC_GameTraceChannel5" "ECR_Overlap")
      (Physics|SetPhysicsLinearVelocity (Variables|/Game/Blueprints/SkullBP.SkullBP_C|GetSkull _output_get) (* _returnvalue 5e+02) false "None")
      (Variables|Default|SetReady false))
    (elif (not (Collision|IsOverlappingActor (Variables|Default|GetCylinder) (Variables|Default|GetFreshSkull) :!class /Script/Engine.PrimitiveComponent))
      (Collision|SetCollisionResponsetoChannel (Variables|/Game/Blueprints/SkullBP.SkullBP_C|GetSkull (Variables|Default|GetFreshSkull)) "ECC_GameTraceChannel5" "ECR_Block")
      (Variables|/Game/Blueprints/SkullBP.SkullBP_C|SetAlive (Variables|Default|GetFreshSkull) true)
      (Variables|Default|SetReady true))))

(fn ConstructionScript)