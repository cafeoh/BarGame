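; Liquid data Blueprint that holds a type, quantity, age, density, color and MRO, with logic to combine two liquids.
; Merge prints an error when the types differ.
; Otherwise it blends each property toward the other liquid using an AAB weight based on both quantities, then adds the other quantity to its own.
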(fn Merge
  (params (Other :type Liquid%20Object%20Reference))
  (if (Utilities|Enum|NotEqual(Enum) (Variables|Default|GetType) (Variables|Liquid_C|GetType Other))
    (Development|PrintString 0 "ERROR: LIQUID MERGE MISMATCH" true true "(R=1.000000,G=0.000000,B=0.113355,A=1.000000)")
    (else
      (Variables|Default|SetAge (Math|Float|Lerp (Variables|Default|GetAge) (Variables|Liquid_C|GetAge Other) (|(A/(A+B)) (Variables|Liquid_C|GetQuantity Other) (Variables|Default|GetQuantity))))
      (Variables|Default|SetDensity (Math|Float|Lerp (Variables|Default|GetDensity) (Variables|Liquid_C|GetDensity Other) (|(A/(A+B)) (Variables|Liquid_C|GetQuantity Other) (Variables|Default|GetQuantity))))
      (Variables|Default|SetColor (Math|Color|Lerp(LinearColor) (Variables|Default|GetColor) (Variables|Liquid_C|GetColor Other) (|(A/(A+B)) (Variables|Liquid_C|GetQuantity Other) (Variables|Default|GetQuantity))))
      (Variables|Default|SetMRO (Math|Color|Lerp(LinearColor) (Variables|Default|GetMRO) (Variables|Liquid_C|GetMRO Other) (|(A/(A+B)) (Variables|Liquid_C|GetQuantity Other) (Variables|Default|GetQuantity))))
      (Variables|Default|SetQuantity (+ (Variables|Default|GetQuantity) (Variables|Liquid_C|GetQuantity Other))))))