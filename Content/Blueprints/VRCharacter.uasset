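; VR player character with floor-origin tracking that moves by axis input and grabs objects with both motion controllers.
; Tick moves it relative to the left controller's forward vector, flattened to the horizontal plane.
; Grip or trigger grabs the first overlapping VRGripInterface actor (or its gripping-capable owner), taking it from the other hand and hiding the gripping hand.
; Release drops held actors with physics and shows the hand again.
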(event EventBeginPlay
  (Class|HeadMountedDisplayFunctionLibrary|SetTrackingOrigin "Floor"))

(event EventTick
  (params (DeltaSeconds :type Float%20%28single-precision%29))
  (bind _leftmotioncontroller (Variables|Default|GetLeftMotionController))
  (bind _returnvalue (Math|Vector|GetForwardVector _leftmotioncontroller))
  (bind _returnvalue_2 (Math|Vector|ProjectVectorontoPlane _returnvalue "0, 0,1.000000"))
  (bind _returnvalue_3 (Math|Vector|Normalize _returnvalue_2))
  (Pawn|Input|AddMovementInput (+ (* _returnvalue_3 (Class|Actor|GetInputAxisKeyValue)) (* (Math|Vector|CrossProduct _returnvalue_3 "0, 0,1.000000") (Class|Actor|GetInputAxisKeyValue))) -1.0 false))

(event Input|KeyboardEvents|MotionControllerLeftGrip1
  (params (Key :type Key%20Structure))
  (bind _leftmotioncontroller (Variables|Default|GetLeftMotionController))
  (bind _rightmotioncontroller (Variables|Default|GetRightMotionController))
  (:Pressed
    (CallFunction|GrabActor (Variables|Default|GetLeftHandGrabSphere) _leftmotioncontroller _rightmotioncontroller))
  (:Released
    (CallFunction|DropAll _leftmotioncontroller _rightmotioncontroller)))

(event Input|KeyboardEvents|MotionControllerLeftTrigger
  (params (Key :type Key%20Structure))
  (bind _leftmotioncontroller (Variables|Default|GetLeftMotionController))
  (bind _rightmotioncontroller (Variables|Default|GetRightMotionController))
  (:Pressed
    (CallFunction|GrabActor (Variables|Default|GetLeftHandGrabSphere) _leftmotioncontroller _rightmotioncontroller))
  (:Released
    (CallFunction|DropAll _leftmotioncontroller _rightmotioncontroller)))

(event Input|KeyboardEvents|MotionControllerRightGrip1
  (params (Key :type Key%20Structure))
  (bind _rightmotioncontroller (Variables|Default|GetRightMotionController))
  (bind _leftmotioncontroller (Variables|Default|GetLeftMotionController))
  (:Pressed
    (CallFunction|GrabActor (Variables|Default|GetRightHandGrabSphere) _rightmotioncontroller _leftmotioncontroller))
  (:Released
    (CallFunction|DropAll _rightmotioncontroller _leftmotioncontroller)))

(event Input|KeyboardEvents|MotionControllerRightTrigger
  (params (Key :type Key%20Structure))
  (bind _rightmotioncontroller (Variables|Default|GetRightMotionController))
  (bind _leftmotioncontroller (Variables|Default|GetLeftMotionController))
  (:Pressed
    (CallFunction|GrabActor (Variables|Default|GetRightHandGrabSphere) _rightmotioncontroller _leftmotioncontroller))
  (:Released
    (CallFunction|DropAll _rightmotioncontroller _leftmotioncontroller)))

(fn ConstructionScript)

(fn DropAll
  (params (MainHand :type Grip%20Motion%20Controller%20Component%20Object%20Reference) (OtherHand :type Grip%20Motion%20Controller%20Component%20Object%20Reference))
  (bind _grippedactorsarray (Class|GripMotionControllerComponent|GetGrippedActors MainHand))
  (for _array_element _grippedactorsarray
    (Class|GripMotionControllerComponent|DropActor MainHand _array_element true "0, 0, 0" "0, 0, 0")
    (Rendering|SetVisibility MainHand true true)))

(fn GrabActor
  (params (SphereCollision :type Sphere%20Component%20Object%20Reference) (MainHand :type Grip%20Motion%20Controller%20Component%20Object%20Reference) (OtherHand :type Grip%20Motion%20Controller%20Component%20Object%20Reference))
  (bind _outactors (Collision|SphereOverlapActors (Transformation|GetWorldLocation SphereCollision) (Variables|/Script/Engine.SphereComponent|GetSphereRadius SphereCollision) (Utilities|Array|MakeArray "ObjectTypeQuery7") 0))
  (bind _array_element (Utilities|Array|ForEachLoopwithBreak _outactors :!label _label)
    (:LoopBody
      (if (Utilities|DoesObjectImplementInterface _array_element "/Script/VRExpansionPlugin.VRGripInterface")
        (bind _grippedactorsarray (Class|GripMotionControllerComponent|GetGrippedActors OtherHand))
        (if (Utilities|Array|ContainsItem _grippedactorsarray (select (Utilities|DoesObjectImplementInterface (Components|GetOwner _array_element) "/Script/VRExpansionPlugin.VRGripInterface") (Components|GetOwner _array_element) _array_element))
          (CallFunction|DropAll OtherHand MainHand))
        (Class|GripMotionControllerComponent|GripActor MainHand (select (Utilities|DoesObjectImplementInterface (Components|GetOwner _array_element) "/Script/VRExpansionPlugin.VRGripInterface") (Components|GetOwner _array_element) _array_element) (Transformation|GetActorTransform (select (Utilities|DoesObjectImplementInterface (Components|GetOwner _array_element) "/Script/VRExpansionPlugin.VRGripInterface") (Components|GetOwner _array_element) _array_element)) false "" "InteractiveCollisionWithPhysics" "NotWhenCollidingOrDoubleGripping" "ForceClientSideMovement" 1.5e+03 2e+02 false)
        (Rendering|SetVisibility MainHand false true)
        (goto _label Break)))))